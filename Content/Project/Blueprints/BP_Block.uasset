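; BP_Block is a networked physics block, simulated on the server and mimicked on clients.
; The server runs physics on the Cube and writes its location and rotation to a Transform variable only while speed exceeds VelocityError, saving bandwidth.
; Clients disable the Cube's collision and, through OnRep_Transform, interpolate it to the received transform with MoveComponentTo in actor-relative space.
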(event `self.ReceiveBeginPlay`
  (`/Engine/EditorBlueprintResources/ActorMacros.Switch Has Authority`
    (:`Authority`
      ;[0 0 0] Physics works only on server side. Client will "simulate" it based on transforms
      (`PrimitiveComponent.SetSimulatePhysics` (`self.Cube`) true))
    (:`Remote`
      (`PrimitiveComponent.SetCollisionEnabled` (`self.Cube`) "NoCollision"))))

(event `self.ReceiveTick`
  (params (DeltaSeconds :type "Float (single-precision)"))
  (bind (_returnvalue_location _returnvalue_rotation) (`KismetMathLibrary.BreakTransform` (`SceneComponent.K2_GetComponentToWorld` (`self.Cube`))))
  ;[0 0 0] Server side: Sync transform if block is moving
  (`/Engine/EditorBlueprintResources/ActorMacros.Switch Has Authority`
    (:`Authority`
      (if (> (`KismetMathLibrary.VSize` (`SceneComponent.GetComponentVelocity` (`self.Cube`))) (`self.VelocityError`))
        (set `self.Transform` (make `LocationForSync` _returnvalue_location _returnvalue_rotation))))))

(event `SimulateMovement`
  (params (Target :type "LocationForSync Structure"))
  (bind _returnvalue (`self.GetTransform`))
  ;[0 0 0] Client side: Move via interpolation
  (`KismetSystemLibrary.MoveComponentTo` (`self.Cube`) (`KismetMathLibrary.InverseTransformLocation` _returnvalue Target_Location) (`KismetMathLibrary.InverseTransformRotation` _returnvalue Target_Rotation)))

(fn `OnRep_Transform`
  (`/Engine/EditorBlueprintResources/ActorMacros.Switch Has Authority`
    (:`Remote`
      (`self.SimulateMovement` (`self.Transform`)))))

(fn `UserConstructionScript`)