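; BP_Shot is a networked physics projectile that flies along a given direction and speed and destroys itself after a short lifetime.
; The server alone simulates physics on the Sphere and, while it moves faster than a threshold, updates a RepNotify Transform each tick.
; Clients disable Sphere collision and, on each replicated update, use MoveComponentTo to interpolate the Sphere toward that transform.
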(event `self.ReceiveBeginPlay`
  (`/Engine/EditorBlueprintResources/ActorMacros.Switch Has Authority`
    (:`Authority`
      (`|ExecutionSequence`
        (:`then_0`
          ;[0 0 0] Physics works only on server side. Client will "simulate" it based on transforms
          (`PrimitiveComponent.SetSimulatePhysics` (`self.Sphere`) true)
          (`PrimitiveComponent.SetAllPhysicsLinearVelocity` (`self.Sphere`) (* (`self.Dir`) (`self.Speed`)) false))
        (:`then_1`
          ;[0 0 0] Lifetime
          (`KismetSystemLibrary.Delay` 3.0)
          (`self.K2_DestroyActor`))))
    (:`Remote`
      (`PrimitiveComponent.SetCollisionEnabled` (`self.Sphere`) "NoCollision"))))

(event `self.ReceiveTick`
  (params (DeltaSeconds :type "Float (single-precision)"))
  (bind (_returnvalue_location _returnvalue_rotation) (`KismetMathLibrary.BreakTransform` (`SceneComponent.K2_GetComponentToWorld` (`self.Sphere`))))
  ;[0 0 0] Server side: Sync transform if projectile is moving
  (`/Engine/EditorBlueprintResources/ActorMacros.Switch Has Authority`
    (:`Authority`
      (if (> (`KismetMathLibrary.VSize` (`SceneComponent.GetComponentVelocity` (`self.Sphere`))) (`self.VelocityError`))
        (set `self.Transform` (make `LocationForSync` _returnvalue_location _returnvalue_rotation))))))

(event `SimulateMovement`
  (params (Target :type "LocationForSync Structure"))
  (bind _returnvalue (`self.GetTransform`))
  ;[0 0 0] Client side: Move via interpolation
  (`KismetSystemLibrary.MoveComponentTo` (`self.Sphere`) (`KismetMathLibrary.InverseTransformLocation` _returnvalue Target_Location) (`KismetMathLibrary.InverseTransformRotation` _returnvalue Target_Rotation)))

(fn `OnRep_Transform`
  (`/Engine/EditorBlueprintResources/ActorMacros.Switch Has Authority`
    (:`Remote`
      (`self.SimulateMovement` (`self.Transform`)))))

(fn `UserConstructionScript`)